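; Bomb actor that the player plants by pressing B nearby to blow open a door.
; Tick checks distance to the first-person character, toggling a text prompt and input within range.
; Pressing B reveals the hidden bomb, then after a delay spawns an explosion with sound and destroys the bomb mesh and the found Door actor.
; The blast triggers slow motion via global time dilation, restored after a short delay.
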(event EventBeginPlay
  (Rendering|SetVisibility (Variables|Default|GetBomb) false false))

(event Collision|EventActorBeginOverlap
  (params (OtherActor :type Actor%20Object%20Reference)))

(event EventTick
  (params (DeltaSeconds :type Float%20%28single-precision%29))
  (bind _textrender (Variables|Default|GetTextRender))
  (bind _asfirst_person_character (Utilities|Casting|CastToFirstPersonCharacter (Game|GetPlayerCharacter 0)))
  (if (< (Transformation|GetDistanceTo _asfirst_person_character) 4e+02)
    (Variables|Default|SetnearBomb true)
    (Rendering|SetVisibility _textrender true false)
    (Input|EnableInput (Game|GetPlayerController 0))
    (else
      (Variables|Default|SetnearBomb false)
      (Rendering|SetVisibility _textrender false false))))

(event Input|ActionEvents|InputActionInteract
  (params (Key :type Key%20Structure :default "None")))

(event Input|KeyboardEvents|B
  (params (Key :type Key%20Structure :default "None"))
  (:Pressed
    (if (Variables|Default|GetnearBomb)
      (Input|DisableInput (Game|GetPlayerController 0))
      (Rendering|SetVisibility (Variables|Default|GetBomb) true false)
      (Utilities|FlowControl|Delay 5.0)
      (CallFunction|Explode)
      (Utilities|FlowControl|Delay 1.5)
      (Utilities|Time|SetGlobalTimeDilation 1.0))))

(fn ConstructionScript)

(fn Explode
  (Game|SpawnActorfromClass "/Game/Blueprints/Explosion.Explosion_C" (Transformation|GetWorldTransform (Variables|Default|GetBomb)) "Undefined" 0 0)
  (Audio|PlaySoundatLocation "/Game/StarterContent/Audio/Explosion01.Explosion01" (Transformation|GetWorldLocation (Variables|Default|GetBomb)) "0, 0, 0" 1.0 1.0 0.0 0 0 0)
  (Components|DestroyComponent (Variables|Default|GetBomb))
  (bind _returnvalue (Actor|GetActorOfClass "/Game/Blueprints/Door.Door_C"))
  (bind _asdoor (Utilities|Casting|CastToDoor _returnvalue))
  (Actor|DestroyActor _asdoor)
  (Variables|Default|SetslowTime true)
  (Utilities|Time|SetGlobalTimeDilation 0.1))