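; Shooting-range target that shows an enemy or civilian material based on IsCivilian and scores hits.
; On overlap it destroys projectiles or rockets, increments the matching kill counter on the CODUI widget, plays a hit or buzzer sound and destroys itself.
; While CanOpen is set, Tick rotates the Target along RotateDirection until an axis-vector check reaches its limit.
; The Z check in RotateAngle compares a constant zero vector, so never matches.
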(event EventBeginPlay
  (bind _target (Variables|Default|GetTarget))
  (if (Variables|Default|GetisCivilian)
    (Rendering|Material|SetMaterial _target 0 "/Game/Materials/CivilianMaterial.CivilianMaterial")
    (else
      (Rendering|Material|SetMaterial _target 0 "/Game/Materials/M_Enemy.M_Enemy"))))

(event Collision|EventActorBeginOverlap
  (params (OtherActor :type Actor%20Object%20Reference))
  (bind _target (Variables|Default|GetTarget))
  (bind _returnvalue (Transformation|GetWorldLocation _target))
  (Utilities|Casting|CastToProjectile_Base OtherActor
    (:then
      (Actor|DestroyActor OtherActor :!label _label))
    (:CastFailed
      (Utilities|Casting|CastToRocket OtherActor
        (:then
          (goto _label))
        (:CastFailed
          _))))
  (bind _foundwidgets (Widget|GetAllWidgetsOfClass "/Game/Blueprints/CODUI.CODUI_C" true))
  (bind _ascodui (Utilities|Casting|CastToCODUI (Utilities|Array|Get(acopy) _foundwidgets)))
  (if (Variables|Default|GetisCivilian)
    (Variables|/Game/Blueprints/CODUI.CODUI_C|SetCiviliansKilled _ascodui (+ (Variables|/Game/Blueprints/CODUI.CODUI_C|GetCiviliansKilled _ascodui) 1))
    (else
      (Variables|/Game/Blueprints/CODUI.CODUI_C|SetTargetsKilled _ascodui (+ (Variables|/Game/Blueprints/CODUI.CODUI_C|GetTargetsKilled _ascodui) 1))))
  (if (Variables|Default|GetisCivilian)
    (Audio|PlaySoundatLocation "/Game/Resources/Wrong_Buzzer_Sound_Effect.Wrong_Buzzer_Sound_Effect" _returnvalue "0, 0, 0" 1.0 1.0 0.0 0 0 0)
    (else
      (Audio|PlaySoundatLocation "/Game/Resources/Critical_Hit__Sound_Effect_.Critical_Hit__Sound_Effect_" _returnvalue "0, 0, 0" 1.0 1.0 0.0 0 0 0)))
  (Actor|DestroyActor))

(event EventTick
  (params (DeltaSeconds :type Float%20%28single-precision%29))
  (if (Variables|Default|GetcanOpen)
    (CallFunction|TurnonTarget)))

(fn ConstructionScript)

(fn TurnonTarget
  (bind _cancontinuerotate (CallFunction|RotateAngle))
  (if (< _cancontinuerotate 1.0)
    (bind _resultrotation (CallFunction|Rotate))
    (Transformation|AddWorldRotation (Variables|Default|GetTarget) _resultrotation false false)))

(fn Rotate
  (bind _rotatedirection (Variables|Default|GetRotateDirection))
  (bind _rotatespeed (Variables|Default|GetRotateSpeed))
  (bind (_x _y _z) (Math|Vector|BreakVector _rotatedirection))
  (return (Math|Rotator|MakeRotator (* _x _rotatespeed) (* _y _rotatespeed) (* _z _rotatespeed))))

(fn RotateAngle
  (if (== (.X (Math|Vector|BreakVector (Variables|Default|GetRotateDirection))) 1.0)
    (return (.Y (Math|Vector|BreakVector (.Y (Math|Rotator|GetAxes (Transformation|GetWorldRotation (Variables|Default|GetTarget)))))))
    (elif (== (.Y (Math|Vector|BreakVector (Variables|Default|GetRotateDirection))) 1.0)
      (return (.Z (Math|Vector|BreakVector (.Z (Math|Rotator|GetAxes (Transformation|GetWorldRotation (Variables|Default|GetTarget)))))))
      (elif (== (.Z (Math|Vector|BreakVector "0, 0, 0")) 1.0)
        (return (.Z (Math|Vector|BreakVector (.Z (Math|Rotator|GetAxes (Transformation|GetWorldRotation (Variables|Default|GetTarget)))))))))))