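; Weapon pickup actor that the player collects with the Interact input, unlocking that weapon on the FirstPersonCharacter.
; Tick measures player distance to show the prompt text and allow interaction within range, re-enabling input every frame.
; Interacting writes the equipped flag and max ammo at WeaponID in the character's arrays, plays a sound and destroys the pickup.
; The construction script applies WeaponMesh; a WeaponID-based mesh switch is left unconnected.
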(event EventBeginPlay
  (Rendering|Components|TextRender|SetText (Variables|Default|GetTextRender) (Utilities|Text|ToText(String) (Variables|Default|GetinteractText))))

(event Collision|EventActorBeginOverlap
  (params (OtherActor :type Actor%20Object%20Reference)))

(event EventTick
  (params (DeltaSeconds :type Float%20%28single-precision%29))
  (Variables|Default|SetcanInteract (< (Math|Vector|Distance(Vector) (Transformation|GetWorldLocation (Variables|Default|GetGun)) (Transformation|GetWorldLocation (Variables|/Script/Engine.Actor|GetRootComponent (Game|GetPlayerCharacter 0)))) 2e+02))
  (Rendering|SetVisibility (Variables|Default|GetTextRender) (Variables|Default|GetcanInteract) false)
  (Input|EnableInput (Game|GetPlayerController 0)))

(event Input|ActionEvents|InputActionInteract
  (params (Key :type Key%20Structure :default "None"))
  (bind _weaponid (Variables|Default|GetweaponID))
  (:Pressed
    (if (Variables|Default|GetcanInteract)
      (bind _asfirst_person_character (Utilities|Casting|CastToFirstPersonCharacter (Game|GetPlayerCharacter 0)))
      (Utilities|Array|SetArrayElem (Variables|/Game/FirstPersonBP/Blueprints/FirstPersonCharacter.FirstPersonCharacter_C|GetweaponEquipped _asfirst_person_character) _weaponid true)
      (Utilities|Array|SetArrayElem (Variables|/Game/FirstPersonBP/Blueprints/FirstPersonCharacter.FirstPersonCharacter_C|GetmaxAmmo _asfirst_person_character) _weaponid (Variables|Default|GetmaxAmmo))
      (Input|DisableInput (Game|GetPlayerController 0))
      (Audio|PlaySoundatLocation "/Game/Resources/PickUpSound.PickUpSound" (Transformation|GetWorldLocation (Variables|Default|GetGun)) "0, 0, 0" 1.0 1.0 0.0 0 0 0)
      (Actor|DestroyActor))))

(fn ConstructionScript
  (Components|StaticMesh|SetStaticMesh (Variables|Default|GetGun) (Variables|Default|GetweaponMesh)))