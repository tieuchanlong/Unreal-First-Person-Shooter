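; RoadBlock is an actor that blocks until its linked ApproachingTarget actors are gone, then destroys itself.
; Every tick it calls CheckApproachingTargetDestroyed, which gets all ApproachingTarget actors and counts those whose ID matches its IDTarget.
; When that count reaches zero, Tick destroys the road block, so a world scan runs every frame.
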(event EventBeginPlay)

(event Collision|EventActorBeginOverlap
  (params (OtherActor :type Actor%20Object%20Reference)))

(event EventTick
  (params (DeltaSeconds :type Float%20%28single-precision%29))
  (bind _targetsdestroyed (CallFunction|CheckApproachingTargetDestroyed))
  (if _targetsdestroyed
    (Actor|DestroyActor)))

(fn ConstructionScript)

(fn CheckApproachingTargetDestroyed
  (Variables|Default|SetcurrentTargetsAvailable 0)
  (bind _outactors (Actor|GetAllActorsOfClass "/Game/Blueprints/ApproachingTarget.ApproachingTarget_C"))
  (for _array_element _outactors
    (bind _asapproaching_target (Utilities|Casting|CastToApproachingTarget _array_element))
    (if (== (Variables|/Game/Blueprints/ApproachingTarget.ApproachingTarget_C|GetID _asapproaching_target) (Variables|Default|GetIDTarget))
      (Variables|Default|SetcurrentTargetsAvailable (+ (Variables|Default|GetcurrentTargetsAvailable) 1))))
  (if (== (Variables|Default|GetcurrentTargetsAvailable) 0)
    (return true)
    (else
      (return false))))