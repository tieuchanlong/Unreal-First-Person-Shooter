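; Mason NPC Blueprint that lets the player talk to him and can end the game afterward.
; Each tick it checks player distance to the standing pose, toggling the interact text and CanInteract.
; TalkToMason shows a random conversation line on the CODUI widget found in the viewport, then clears it after a delay.
; If CanEndGame is set, it then opens the end screen, shows the cursor and pauses the game.
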(event Custom|Talk%20To%20Mason
  (if (Variables|Default|GetcanInteract)
    (Variables|Default|SetcurrentConvInd (Math|Random|RandomIntegerinRange 0 (- (Utilities|Array|Length (Variables|Default|GetConversations)) 1)))
    (bind _foundwidgets (Widget|GetAllWidgetsOfClass "/Game/Blueprints/CODUI.CODUI_C" true))
    (bind _ascodui (Utilities|Casting|CastToCODUI (Utilities|Array|Get(acopy) _foundwidgets)))
    (Variables|/Game/Blueprints/CODUI.CODUI_C|SetConversation _ascodui (Utilities|Array|Get(acopy) (Variables|Default|GetConversations) (Variables|Default|GetcurrentConvInd)))
    (Utilities|FlowControl|Delay 5.0)
    (Variables|/Game/Blueprints/CODUI.CODUI_C|SetConversation _ascodui "")
    (if (Variables|Default|GetcanEndGame)
      (bind _returnvalue (UserInterface|CreateWidget "/Game/Blueprints/COD_End_UI_BP.COD_End_UI_BP_C"))
      (bind _output_get (Variables|Default|SetEndGameRef _returnvalue))
      (Variables|/Script/Engine.PlayerController|SetbShowMouseCursor (Game|GetPlayerController 0) true)
      (UserInterface|Viewport|AddtoViewport _output_get 0)
      (Game|SetGamePaused true))))

(event EventBeginPlay)

(event Collision|EventActorBeginOverlap
  (params (OtherActor :type Actor%20Object%20Reference)))

(event EventTick
  (params (DeltaSeconds :type Float%20%28single-precision%29))
  (bind _interacttext (Variables|Default|GetInteractText))
  (bind _nearplayer (CallFunction|CheckNearPlayer))
  (Variables|Default|SetcanInteract _nearplayer)
  (if _nearplayer
    (Rendering|SetVisibility _interacttext true false)
    (else
      (Rendering|SetVisibility _interacttext false false))))

(fn ConstructionScript)

(fn CheckNearPlayer
  (return (< (Math|Vector|Distance(Vector) (Transformation|GetWorldLocation (Variables|Default|GetMason_Standing_Pose)) (Transformation|GetWorldLocation (Variables|/Script/Engine.Actor|GetRootComponent (Game|GetPlayerCharacter 0)))) 3e+02)))