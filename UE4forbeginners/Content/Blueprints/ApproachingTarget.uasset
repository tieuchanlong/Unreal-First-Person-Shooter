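; Shooting target that flips up, slides along its right vector, then flips down and destroys itself on reaching a MovingTargetStopBlock.
; Tick runs these phases as a boolean state machine, gated by CanOpen and a one-time startup delay.
; Overlapping projectiles or rockets are destroyed along with the target, incrementing TargetsKilled on the CODUI widget found by class lookup.
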(event EventBeginPlay)

(event Collision|EventActorBeginOverlap
  (params (OtherActor :type Actor%20Object%20Reference))
  (Utilities|Casting|CastToMovingTargetStopBlock OtherActor
    (:then
      (Variables|Default|SetmovingTarget false)
      (Variables|Default|SetturningOffTarget true))
    (:CastFailed
      (bind _asprojectile_base (Utilities|Casting|CastToProjectile_Base OtherActor)
        (:then
          (Actor|DestroyActor _asprojectile_base)
          (CallFunction|AddTargetKilled))
        (:CastFailed
          (bind _asrocket (Utilities|Casting|CastToRocket OtherActor))
          (Actor|DestroyActor _asrocket)
          (CallFunction|AddTargetKilled))))))

(event EventTick
  (params (DeltaSeconds :type Float%20%28single-precision%29))
  (if (Variables|Default|GetcanOpen)
    (if (Variables|Default|GetalreadyDelay)
      (if (Variables|Default|GetcanActivate)
        (if (Variables|Default|GetturningOnTarget)
          (CallFunction|TurnonTarget)
          (elif (Variables|Default|GetmovingTarget)
            (CallFunction|MoveTarget)
            (elif (Variables|Default|GetturningOffTarget)
              (CallFunction|TurnOffTarget)
              (else
                (Actor|DestroyActor))))))
      (else
        (Utilities|FlowControl|Delay (Variables|Default|GetdelayTime))
        (Variables|Default|SetcanActivate true)
        (Variables|Default|SetalreadyDelay true)))))

(fn ConstructionScript)

(fn TurnonTarget
  (if (< -1.0 (.Y (Math|Vector|BreakVector (.Y (Math|Rotator|GetAxes (Transformation|GetWorldRotation (Variables|Default|GetStaticMesh)))))))
    (Transformation|AddWorldRotation (Variables|Default|GetStaticMesh) (Math|Rotator|MakeRotator (Variables|Default|GetRotateSpeed) 0.0 0.0) false false)
    (else
      (Variables|Default|SetturningOnTarget false)
      (Variables|Default|SetmovingTarget true))))

(fn TurnOffTarget
  (if (> 0.0 (.Y (Math|Vector|BreakVector (.Y (Math|Rotator|GetAxes (Transformation|GetWorldRotation (Variables|Default|GetStaticMesh)))))))
    (Transformation|AddWorldRotation (Variables|Default|GetStaticMesh) (Math|Rotator|MakeRotator (* (Variables|Default|GetRotateSpeed) -1.0) 0.0 0.0) false false)
    (else
      (Variables|Default|SetturningOffTarget false)
      (Actor|DestroyActor))))

(fn MoveTarget
  (Transformation|SetWorldLocation (Variables|Default|GetStaticMesh) (+ (Transformation|GetActorLocation) (* (Transformation|GetActorRightVector) (Variables|Default|GetMoveSpeed))) false false))

(fn AddTargetKilled
  (bind _foundwidgets (Widget|GetAllWidgetsOfClass "/Game/Blueprints/CODUI.CODUI_C" true))
  (bind _ascodui (Utilities|Casting|CastToCODUI (Utilities|Array|Get(acopy) _foundwidgets)))
  (Variables|/Game/Blueprints/CODUI.CODUI_C|SetTargetsKilled _ascodui (+ (Variables|/Game/Blueprints/CODUI.CODUI_C|GetTargetsKilled _ascodui) 1))
  (Actor|DestroyActor))