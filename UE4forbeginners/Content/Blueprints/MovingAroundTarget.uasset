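; Moving target actor that can turn on, then travel back and forth between direction-switching blocks.
; TurnOnTarget is meant to roll the mesh upright, but its axis check reads a zero rotator, so it switches straight to the moving state.
; MoveTarget offsets the mesh along actor forward, and overlapping a TargetSwitchingDirectionBlock negates MoveSpeed.
; Tick is empty; nothing here calls either motion function.
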(event EventBeginPlay)

(event Collision|EventActorBeginOverlap
  (params (OtherActor :type Actor%20Object%20Reference))
  (Utilities|Casting|CastToTargetSwitchingDirectionBlock OtherActor)
  (CallFunction|ChangeDirection))

(event EventTick
  (params (DeltaSeconds :type Float%20%28single-precision%29)))

(fn ConstructionScript)

(fn TurnonTarget
  (if (< (.Y (Math|Vector|BreakVector (.Y (Math|Rotator|GetAxes "0, 0, 0")))) 1.0)
    (Transformation|AddWorldRotation (Variables|Default|GetStaticMesh) (Math|Rotator|MakeRotator (Variables|Default|GetRotateSpeed) 0.0 0.0) false false)
    (else
      (Variables|Default|SetturningOnTarget false)
      (Variables|Default|SetmovingTarget true))))

(fn MoveTarget
  (Transformation|SetWorldLocation (Variables|Default|GetStaticMesh) (+ (Transformation|GetActorLocation) (* (Transformation|GetActorForwardVector) (Variables|Default|GetMoveSpeed))) false false))

(fn ChangeDirection
  (Variables|Default|SetmoveSpeed (* (Variables|Default|GetmoveSpeed) -1.0)))